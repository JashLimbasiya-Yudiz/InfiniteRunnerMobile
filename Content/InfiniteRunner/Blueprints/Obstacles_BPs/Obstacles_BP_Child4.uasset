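; Obstacle child Blueprint for the infinite runner, whose construction script only calls the parent's.
; Its event graph holds player-hit logic with no event driving it, so that logic never runs here.
; The unused chain would spend the game mode's shield, play a break sound and destroy the obstacle, or call the character's Death when unshielded.
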(fn `UserConstructionScript`
  (`parent.UserConstructionScript`))