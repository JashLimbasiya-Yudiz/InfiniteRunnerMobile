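; Recyclable three-lane floor tile for the infinite runner that spawns its own obstacles and pickups.
; ConstructFloor randomly fills lane spawn points with child actors: coin rows, occasional special pickups timed by a GameMode counter, and obstacles, capping the blocking type at two.
; When the player overlaps Box, it raises run speed, updates score and saved high score, then rebuilds the GameMode's first floor and moves it to the track's end.
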(event `self.Box.OnComponentBeginOverlap`
  (params (OverlappedComponent :type "PrimitiveComponent Object Reference") (OtherActor :type "Actor Object Reference") (OtherComp :type "PrimitiveComponent Object Reference") (OtherBodyIndex :type Integer) (bFromSweep :type Boolean) (SweepResult :type "HitResult Structure (by ref)"))
  (if (== OtherActor (`GameplayStatics.GetPlayerCharacter` 0))
    (`self.Update Speed`)
    (`self.Update Score`)
    (`KismetSystemLibrary.Delay` 0.01)
    (`self.Update Map`)))

(fn `Construct Floor`
  (for _index (range 3)
    (`self.Generate Obstacle Spawn Points` _index)
    (`self.Generate Coins Spawn Points` _index))
  (`self.Increment Special Spawn Time`)
  (`self.SpawnCollectibles`)
  (`self.SpawnObstacles`))

(fn `DestroyChildActors`
  (bind _childactors (`self.ChildActors`))
  (for _array_element _childactors
    (`ActorComponent.K2_DestroyComponent` _array_element))
  (`KismetArrayLibrary.Array_Clear` _childactors)
  (`KismetArrayLibrary.Array_Clear` (`self.ObstacleSpawnPoints`))
  (`KismetArrayLibrary.Array_Clear` (`self.CoinsSpawnPoints`)))

(fn `Generate Coins Spawn Points`
  (params (LaneIndex :type Integer))
  (bind _returnvalue (`AddComponent|NODE_AddArrowComponent-1` :`RelativeTransform` (`KismetMathLibrary.MakeTransform` (`KismetMathLibrary.MakeVector` 300.0 (`|GetArrayItem` (`self.LanePosition`) LaneIndex)))))
  (`KismetArrayLibrary.Array_Add` (`self.CoinsSpawnPoints`) (`SceneComponent.K2_GetComponentToWorld` _returnvalue)))

(fn `Generate Obstacle Spawn Points`
  (params (LaneIndex :type Integer))
  (bind _returnvalue (`AddComponent|NODE_AddArrowComponent-0` :`RelativeTransform` (`KismetMathLibrary.MakeTransform` (`KismetMathLibrary.MakeVector` 1800.0 (`|GetArrayItem` (`self.LanePosition`) LaneIndex)))))
  (`KismetArrayLibrary.Array_Add` (`self.ObstacleSpawnPoints`) (`SceneComponent.K2_GetComponentToWorld` _returnvalue)))

(fn `Increment Special Spawn Time`
  (bind _asthird_person_game_mode (cast `/Game/InfiniteRunner/ThirdPersonBP/Blueprints/ThirdPersonGameMode` (`GameplayStatics.GetGameMode`)))
  (set `/Game/InfiniteRunner/ThirdPersonBP/Blueprints/ThirdPersonGameMode.SpecialSpawnTime` (+ (`/Game/InfiniteRunner/ThirdPersonBP/Blueprints/ThirdPersonGameMode.SpecialSpawnTime` _asthird_person_game_mode) 1) _asthird_person_game_mode))

(fn `SpawnCollectibles`
  (bind _returnvalue (`KismetMathLibrary.RandomIntegerInRange` 0 20))
  (for _array_element (`self.CoinsSpawnPoints`)
    (if (and (== (mod _returnvalue 2) 0) (> _returnvalue 10))
      (for _index (range 5)
        (if (< _index 4)
          (bind (_returnvalue_location _returnvalue_rotation _returnvalue_scale) (`KismetMathLibrary.BreakTransform` (`KismetMathLibrary.MakeRelativeTransform` _array_element (`self.GetTransform`))))
          (bind _returnvalue_2 (`KismetMathLibrary.Conv_IntToDouble` (* _index 200)))
          (bind _returnvalue_3 (`AddComponent|NODE_AddChildActorComponent-4` :`RelativeTransform` (`KismetMathLibrary.MakeTransform` (+ _returnvalue_location (`KismetMathLibrary.MakeVector` _returnvalue_2)) _returnvalue_rotation _returnvalue_scale) :!label _label))
          (`KismetArrayLibrary.Array_Add` (`self.ChildActors`) _returnvalue_3)
          (else
            (bind _asthird_person_game_mode (cast `/Game/InfiniteRunner/ThirdPersonBP/Blueprints/ThirdPersonGameMode` (`GameplayStatics.GetGameMode`)))
            (if (> (`/Game/InfiniteRunner/ThirdPersonBP/Blueprints/ThirdPersonGameMode.SpecialSpawnTime` _asthird_person_game_mode) 11)
              (switch `int` (`KismetMathLibrary.RandomIntegerInRange` 0 6)
                (:`0`
                  (bind (_returnvalue_location_2 _returnvalue_rotation_2 _returnvalue_scale_2) (`KismetMathLibrary.BreakTransform` (`KismetMathLibrary.MakeRelativeTransform` _array_element (`self.GetTransform`))))
                  (bind _returnvalue_4 (`KismetMathLibrary.MakeTransform` (+ _returnvalue_location_2 (`KismetMathLibrary.MakeVector` _returnvalue_2)) _returnvalue_rotation_2 _returnvalue_scale_2))
                  (bind _returnvalue_5 (`AddComponent|NODE_AddChildActorComponent-5` :`RelativeTransform` _returnvalue_4 :!label _label_2))
                  (`KismetArrayLibrary.Array_Add` (`self.ChildActors`) _returnvalue_5))
                (:`1`
                  (goto _label_2))
                (:`2`
                  (bind _returnvalue_6 (`AddComponent|NODE_AddChildActorComponent-6` :`RelativeTransform` _returnvalue_4 :!label _label_3))
                  (`KismetArrayLibrary.Array_Add` (`self.ChildActors`) _returnvalue_6))
                (:`3`
                  (goto _label_3))
                (:`4`
                  (bind _returnvalue_7 (`AddComponent|NODE_AddChildActorComponent-7` :`RelativeTransform` _returnvalue_4 :!label _label_4))
                  (`KismetArrayLibrary.Array_Add` (`self.ChildActors`) _returnvalue_7))
                (:`5`
                  (goto _label_4))
                (:`6`
                  (bind _returnvalue_8 (`AddComponent|NODE_AddChildActorComponent-8` :`RelativeTransform` _returnvalue_4))
                  (`KismetArrayLibrary.Array_Add` (`self.ChildActors`) _returnvalue_8)))
              (set `/Game/InfiniteRunner/ThirdPersonBP/Blueprints/ThirdPersonGameMode.SpecialSpawnTime` 0 _asthird_person_game_mode)
              (else
                (goto _label)))))))))

(fn `SpawnObstacles`
  (set `self.BlockedObstacleCount` 0)
  (for _array_element (`self.ObstacleSpawnPoints`)
    (if (`KismetMathLibrary.RandomBool`)
      (switch `int` (`KismetMathLibrary.RandomIntegerInRange` 0 3)
        (:`0`
          (bind _returnvalue (`KismetMathLibrary.MakeRelativeTransform` _array_element (`self.GetTransform`)))
          (bind _returnvalue_2 (`AddComponent|NODE_AddChildActorComponent-0` :`RelativeTransform` _returnvalue))
          (`KismetArrayLibrary.Array_Add` (`self.ChildActors`) _returnvalue_2))
        (:`1`
          (bind _returnvalue_3 (`AddComponent|NODE_AddChildActorComponent-1` :`RelativeTransform` _returnvalue))
          (`KismetArrayLibrary.Array_Add` (`self.ChildActors`) _returnvalue_3))
        (:`2`
          (bind _returnvalue_4 (`AddComponent|NODE_AddChildActorComponent-2` :`RelativeTransform` _returnvalue))
          (`KismetArrayLibrary.Array_Add` (`self.ChildActors`) _returnvalue_4))
        (:`3`
          (if (< (`self.BlockedObstacleCount`) 2)
            (bind _returnvalue_5 (`AddComponent|NODE_AddChildActorComponent-3` :`RelativeTransform` _returnvalue))
            (`KismetArrayLibrary.Array_Add` (`self.ChildActors`) _returnvalue_5)
            (`/Engine/EditorBlueprintResources/StandardMacros.IncrementInt` (`self.BlockedObstacleCount`))))))))

(fn `Update Map`
  (bind _asthird_person_game_mode (cast `/Game/InfiniteRunner/ThirdPersonBP/Blueprints/ThirdPersonGameMode` (`GameplayStatics.GetGameMode`)))
  (bind _floors (`/Game/InfiniteRunner/ThirdPersonBP/Blueprints/ThirdPersonGameMode.Floors` _asthird_person_game_mode))
  (bind _output (`|GetArrayItem` _floors (`/Game/InfiniteRunner/ThirdPersonBP/Blueprints/ThirdPersonGameMode.FirstFloorIndex` _asthird_person_game_mode)))
  (`self.DestroyChildActors` _output)
  (`self.Construct Floor` _output)
  (`self.K2_SetActorLocation` _output (`SceneComponent.K2_GetComponentLocation` (`/Game/InfiniteRunner/Blueprints/Floor_BP.NextFloor` (`|GetArrayItem` _floors (`/Game/InfiniteRunner/ThirdPersonBP/Blueprints/ThirdPersonGameMode.LastFloorIndex` _asthird_person_game_mode)))) false true)
  (`/Game/InfiniteRunner/ThirdPersonBP/Blueprints/ThirdPersonGameMode.UpdateFirstAndLastFloorIndex` _asthird_person_game_mode))

(fn `Update Score`
  (bind _asthird_person_game_mode (cast `/Game/InfiniteRunner/ThirdPersonBP/Blueprints/ThirdPersonGameMode` (`GameplayStatics.GetGameMode`)))
  (if (`/Game/InfiniteRunner/ThirdPersonBP/Blueprints/ThirdPersonGameMode.Is10xOn` _asthird_person_game_mode)
    (bind _currentscore (`/Game/InfiniteRunner/ThirdPersonBP/Blueprints/ThirdPersonGameMode.CurrentScore` _asthird_person_game_mode))
    (set `/Game/InfiniteRunner/ThirdPersonBP/Blueprints/ThirdPersonGameMode.CurrentScore` (+ _currentscore 10) _asthird_person_game_mode)
    (else
      (set `/Game/InfiniteRunner/ThirdPersonBP/Blueprints/ThirdPersonGameMode.CurrentScore` (+ _currentscore 1) _asthird_person_game_mode)))
  (bind _returnvalue (`GameplayStatics.LoadGameFromSlot` "SaveGame"))
  (bind _asinfinite_runner_save_game (cast `/Game/InfiniteRunner/Blueprints/InfiniteRunnerSaveGame` _returnvalue))
  (bind _currentscore_2 (`/Game/InfiniteRunner/ThirdPersonBP/Blueprints/ThirdPersonGameMode.CurrentScore` _asthird_person_game_mode))
  (if (< (`/Game/InfiniteRunner/Blueprints/InfiniteRunnerSaveGame.HighScore` _asinfinite_runner_save_game) _currentscore_2)
    (set `/Game/InfiniteRunner/Blueprints/InfiniteRunnerSaveGame.HighScore` _currentscore_2 _asinfinite_runner_save_game)
    (`GameplayStatics.SaveGameToSlot` _asinfinite_runner_save_game "SaveGame")))

(fn `Update Speed`
  (bind _asthird_person_character (cast `/Game/InfiniteRunner/ThirdPersonBP/Blueprints/ThirdPersonCharacter` (`GameplayStatics.GetPlayerCharacter` 0)))
  (bind _charactermovement (`Character.CharacterMovement` _asthird_person_character))
  (set `CharacterMovementComponent.MaxWalkSpeed` (`KismetMathLibrary.FClamp` (+ (`CharacterMovementComponent.MaxWalkSpeed` _charactermovement) 3.3) 0.0 3333.0) _charactermovement))

(fn `UserConstructionScript`
  (`self.Construct Floor`))